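; Player interaction component that detects interactable and collectible actors in view and handles interacting with or collecting them.
; A looping timer, which can be paused and resumed, line-traces from the camera and shows or clears a HUD prompt based on the hit actor's tags.
; Interact sends the matching message to that actor, then clears the prompt.
; An optional FacingCharacter tag adds a dot-product facing check for interactables.
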(event EventBeginPlay
  (Utilities|Time|SetTimerbyFunctionName 0 "CheckForInteraction" 0.1 true))

(fn CheckforInteraction
  (bind _playercameracomp (Variables|Default|GetPlayerCameraComp))
  (bind _returnvalue (Transformation|GetWorldLocation _playercameracomp))
  (bind (_outhit _returnvalue_2) (Collision|LineTraceByChannel _returnvalue (+ _returnvalue (* (Math|Vector|GetForwardVector (Variables|Default|GetPlayerCameraComp)) (Variables|Default|GetInteractionDistance))) "TraceTypeQuery3" false 0 "ForDuration"))
  (bind _output_get (Variables|Default|SetCanBeInteractedWith? _returnvalue_2))
  (if _output_get
    (if (!= (.HitActor (Collision|BreakHitResult _outhit)) (Variables|Default|GetLookAtActor))
      (bind _output_get_2 (Variables|Default|SetLookAtActor (.HitActor (Collision|BreakHitResult _outhit))))
      (if (Utilities|Array|IsNotEmpty (Variables|/Script/Engine.Actor|GetTags _output_get_2))
        (for _array_element (Variables|/Script/Engine.Actor|GetTags _output_get_2)
          (switch name _array_element
            (:Interactable
              (if (CallFunction|InteractableCheck)
                (Default|ShowHideInteractMessage (Variables|/Game/BPs/PlayerRelated/PlayerSystems/BP_AC_UIManager.BP_AC_UIManager_C|GetPlayerHUD (Variables|Default|GetPlayerUIManager)) "Press E To Interact")))
            (:Collectible
              (Default|ShowHideInteractMessage (Variables|/Game/BPs/PlayerRelated/PlayerSystems/BP_AC_UIManager.BP_AC_UIManager_C|GetPlayerHUD (Variables|Default|GetPlayerUIManager)) "Press E To Collect"))))
        (else
          (Default|ShowHideInteractMessage (Variables|/Game/BPs/PlayerRelated/PlayerSystems/BP_AC_UIManager.BP_AC_UIManager_C|GetPlayerHUD (Variables|Default|GetPlayerUIManager)) :!label _label))))
    (else
      (Variables|Default|SetLookAtActor 0)
      (goto _label))))

(fn ContinueInteractionCheck
  (Class|KismetSystemLibrary|UnPauseTimer 0 "CheckForInteraction"))

(fn HoldInteractionCheck
  (Class|KismetSystemLibrary|PauseTimer 0 "CheckForInteraction"))

(fn InteractableCheck
  (if (Utilities|Array|ContainsItem (Variables|/Script/Engine.Actor|GetTags (Variables|Default|GetLookAtActor)) "FacingCharacter")
    (return (>= (Math|Vector|DotProduct (Transformation|GetActorForwardVector (Game|GetPlayerCharacter 0)) (* (Transformation|GetActorForwardVector (Variables|Default|GetLookAtActor)) -1.0)) 0.8))
    (else
      (return true))))

(fn Interact
  (bind _lookatactor (Variables|Default|GetLookAtActor)
    (:then
      (if (Utilities|Array|IsNotEmpty (Variables|/Script/Engine.Actor|GetTags _lookatactor))
        (for _array_element (Variables|/Script/Engine.Actor|GetTags _lookatactor)
          (switch name _array_element
            (:Interactable
              (if (CallFunction|InteractableCheck)
                (Class|BPIInteraction|Interact(Message) (Variables|Default|GetLookAtActor))
                (Development|PrintString "Interactable")))
            (:Collectible
              (Class|BPIInteraction|Collect(Message) (Variables|Default|GetLookAtActor))
              (Development|PrintString "Collectible"))))
        (CallFunction|ClearInteractionUI)))
    (:else)))

(fn ClearInteractionUI
  (Variables|Default|SetLookAtActor 0)
  (Default|ShowHideInteractMessage (Variables|/Game/BPs/PlayerRelated/PlayerSystems/BP_AC_UIManager.BP_AC_UIManager_C|GetPlayerHUD (Variables|Default|GetPlayerUIManager))))