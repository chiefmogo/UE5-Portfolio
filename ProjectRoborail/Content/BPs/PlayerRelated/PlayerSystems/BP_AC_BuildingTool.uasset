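; Player component that runs the build mode for placing buildables on train compartments.
; Entering build mode shows compartment grids and starts a looping timer that line-traces from the view to tagged build surfaces.
; Hits snap to the compartment's local grid, where footprint bounds and occupancy drive the preview actor's validity.
; Confirming checks unlock, build limit and inventory cost, then spawns and attaches the buildable, marks its cells occupied and exits.
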(event EventBeginPlay)

(event EventTick
  (params (DeltaSeconds :type Float%20%28single-precision%29)))

(fn EnterBuildMode
  (Variables|State|SetIsBuildMode true)
  (bind _trainref (Variables|References|GetTrainRef)
    (:then
      (for _array_element (Variables|/Game/BPs/Train/BP_Train.BP_Train_C|GetActiveTrainCompartments _trainref)
        (Utilities|IsValid _array_element
          (:Is%20Valid
            (if (Variables|/Game/BPs/Train/BP_TrainCompartment.BP_TrainCompartment_C|GetBuildableCompartment? _array_element)
              (Development|SetHiddeninGame (Variables|/Game/BPs/Train/BP_TrainCompartment.BP_TrainCompartment_C|GetGridVisual _array_element) false false)
              (Default|ShowHideBuildables (Variables|/Game/BPs/PlayerRelated/BP_Player.BP_Player_C|GetUI%20Manager%20Component (.AsBP%20Player (Utilities|Casting|CastToBP_Player (Components|GetOwner)))) (Variables|State|GetIsBuildMode))))))
      (CallFunction|StartBuildUpdateLoop))
    (:else)))

(fn ExitBuildMode
  (Variables|State|SetIsBuildMode false)
  (Variables|State|SetPlacementValid false)
  (Variables|State|SetSelectedBuildableClass 0)
  (Variables|References|SetTargetCompartment 0)
  (bind _previewactor (Variables|References|GetPreviewActor)
    (:then
      (Rendering|SetActorHiddenInGame _previewactor true))
    (:else
      _))
  (Variables|References|SetPreviewActor 0)
  (bind _trainref (Variables|References|GetTrainRef)
    (:then
      (for _array_element (Variables|/Game/BPs/Train/BP_Train.BP_Train_C|GetActiveTrainCompartments _trainref)
        (Utilities|IsValid _array_element
          (:Is%20Valid
            (if (Variables|/Game/BPs/Train/BP_TrainCompartment.BP_TrainCompartment_C|GetBuildableCompartment? _array_element)
              (Development|SetHiddeninGame (Variables|/Game/BPs/Train/BP_TrainCompartment.BP_TrainCompartment_C|GetGridVisual _array_element) true false)
              (Default|ShowHideBuildables (Variables|/Game/BPs/PlayerRelated/BP_Player.BP_Player_C|GetUI%20Manager%20Component (.AsBP%20Player (Utilities|Casting|CastToBP_Player (Components|GetOwner)))) (Variables|State|GetIsBuildMode))))))
      (CallFunction|StopBuildUpdateLoop))
    (:else)))

(fn SelectBuildable
  (params (BuildableClass :type BP%20Buildables%20Master%20Class%20Reference))
  (Variables|State|SetSelectedBuildableClass BuildableClass)
  (bind _previewactor (Variables|References|GetPreviewActor)
    (:then
      (Rendering|SetActorHiddenInGame _previewactor false))
    (:else
      (bind _returnvalue (Game|SpawnActorfromClass "/Game/BPs/Building/BP_BuildPreviewActor.BP_BuildPreviewActor_C" (Math|Transform|MakeTransform "0, 0, 0" "0, 0, 0" "1.000000,1.000000,1.000000") "Undefined" "MultiplyWithRoot" 0 0))
      (bind _output_get (Variables|References|SetPreviewActor _returnvalue))))
  (Default|SetPreviewMesh _output_get (.PreviewMesh (Utilities|GetClassDefaults (Variables|State|GetSelectedBuildableClass)))))

(fn StartBuildUpdateLoop
  (bind _returnvalue (Utilities|Time|SetTimerbyFunctionName 0 "UpdatePreview" 0.03 true))
  (Variables|State|SetBuildUpdateTimerHandle _returnvalue))

(fn StopBuildUpdateLoop
  (Utilities|Time|ClearandInvalidateTimerbyHandle (Variables|State|GetBuildUpdateTimerHandle)))

(fn UpdatePreview
  (bind _returnvalue (Game|GetPlayerController 0))
  (bind _gridcellsize (Variables|Grid|GetGridCellSize))
  (bind _selectedbuildableclass (Variables|State|GetSelectedBuildableClass))
  (bind (_location _rotation) (Pawn|GetPlayerViewPoint _returnvalue))
  (bind (_needsinteractionui _buildableunlocked_ _buildablename _builtnumber _maxbuildsallowed _buildcosts _footprintextent _mi_ghost_valid _mi_ghost_invalid _mi_ghost_nofunds _rotationsnapdegrees _previewmesh _footprintcellsx _footprintcellsy) (Utilities|GetClassDefaults _selectedbuildableclass))
  (bind _returnvalue_2 (/ _gridcellsize 2.0))
  (Variables|References|SetHasValidBuildHit false)
  (if (Variables|State|GetIsBuildMode)
    (Variables|State|GetSelectedBuildableClass
      (:then
        (Variables|References|GetPreviewActor
          (:then
            (Variables|References|GetTrainRef
              (:then
                (bind (_outhit _returnvalue_3) (Collision|LineTraceByChannel _location (+ _location (* (Math|Vector|GetForwardVector _rotation) 5e+03)) "TraceTypeQuery4" false 0 "None"))
                (if _returnvalue_3
                  (if (Components|ComponentHasTag (.HitComponent (Collision|BreakHitResult _outhit)) "BuildSurface")
                    (bind _asbp_train_compartment (Utilities|Casting|CastToBP_TrainCompartment (Components|GetOwner (.HitComponent (Collision|BreakHitResult _outhit)))))
                    (bind _output_get (LocalVariables|SetHitCompartment _asbp_train_compartment))
                    (bind _buildablecompartment (Default|IsBuildable _output_get))
                    (if _buildablecompartment
                      (Variables|References|SetHasValidBuildHit true)
                      (bind _output_get_2 (Variables|References|SetTargetCompartment (LocalVariables|GetHitCompartment)))
                      (bind _gridorigintransform (Default|GetGridOriginTransform _output_get_2))
                      (bind _output_get_3 (LocalVariables|SetGridT _gridorigintransform))
                      (bind _output_get_4 (LocalVariables|SetLocalHit (Math|Transform|InverseTransformLocation _output_get_3 (.Location (Collision|BreakHitResult _outhit)))))
                      (bind _output_get_5 (LocalVariables|SetCellX (Math|Float|Round (/ (.x _output_get_4) (Variables|Grid|GetGridCellSize)))))
                      (Variables|Grid|SetLastCellX _output_get_5)
                      (bind _output_get_6 (LocalVariables|SetCellY (Math|Float|Round (/ (.y _output_get_4) (Variables|Grid|GetGridCellSize)))))
                      (Variables|Grid|SetLastCellY _output_get_6)
                      (LocalVariables|SetSnappedWorld (Math|Transform|TransformLocation (LocalVariables|GetGridT) (Math|Vector|MakeVector (+ (* (LocalVariables|GetCellX) _gridcellsize) _returnvalue_2) (+ (* _gridcellsize (LocalVariables|GetCellY)) _returnvalue_2) 0.0)))
                      (LocalVariables|SetBuildableFootprintCellX _footprintcellsx)
                      (LocalVariables|SetBuildableFootprintCellY _footprintcellsy)
                      (bind _withinbounds (Default|IsAreaWithinBounds (Variables|References|GetTargetCompartment)))
                      (if _withinbounds
                        (bind _free (Default|IsAreaFree? (Variables|References|GetTargetCompartment) (LocalVariables|GetCellX) (LocalVariables|GetCellY) (LocalVariables|GetBuildableFootprintCellX) (LocalVariables|GetBuildableFootprintCellY)))
                        (if (Variables|References|GetHasValidBuildHit)
                          (Variables|State|SetPlacementValid _free)
                          (else
                            (Variables|State|SetPlacementValid false)))
                        (Default|SetValidState (Variables|References|GetPreviewActor) (Variables|State|GetPlacementValid))
                        (LocalVariables|SetYaw (* (Variables|Grid|GetRotationIndex) 90))
                        (Transformation|SetActorLocationAndRotation (Variables|References|GetPreviewActor) (LocalVariables|GetSnappedWorld) (Math|Rotator|MakeRotator 0.0 (LocalVariables|GetYaw) 0.0))
                        (Rendering|SetActorHiddenInGame (Variables|References|GetPreviewActor) false)
                        (Variables|Grid|SetLastSnappedTransform (Math|Transform|MakeTransform (LocalVariables|GetSnappedWorld) (Math|Rotator|MakeRotator 0.0 (LocalVariables|GetYaw) 0.0))))))))
              (:else
                (return))))
          (:else
            (return))))
      (:else
        (return)))
    (else
      (return))))

(fn ConfirmBuild
  (bind _selectedbuildableclass (Variables|State|GetSelectedBuildableClass))
  (bind _selectedbuildableclass_2 (Variables|State|GetSelectedBuildableClass))
  (bind (_needsinteractionui _buildableunlocked_ _buildablename _builtnumber _maxbuildsallowed _buildcosts _footprintextent _mi_ghost_valid _mi_ghost_invalid _mi_ghost_nofunds _rotationsnapdegrees _previewmesh _footprintcellsx _footprintcellsy) (Utilities|GetClassDefaults _selectedbuildableclass_2))
  (bind (_needsinteractionui_2 _buildableunlocked__2 _buildablename_2 _builtnumber_2 _maxbuildsallowed_2 _buildcosts_2) (Utilities|GetClassDefaults _selectedbuildableclass))
  (if (Variables|State|GetIsBuildMode)
    (Variables|State|GetSelectedBuildableClass
      (:then
        (Variables|References|GetTargetCompartment
          (:then
            (if (Variables|State|GetPlacementValid)
              (if _buildableunlocked__2
                (bind _count (Default|GetBuiltCount (Variables|References|GetTrainRef) (Variables|State|GetSelectedBuildableClass)))
                (bind _output_get (LocalVariables|SetCurrentCount _count))
                (if (< _output_get _maxbuildsallowed_2)
                  (if (Default|CanAffordCosts (Actor|GetComponentbyClass (Components|GetOwner) "/Game/BPs/CommonSystems/Inventory/BP_AC_Inventory.BP_AC_Inventory_C") _buildcosts_2)
                    (bind _returnvalue (Game|SpawnActorfromClass (Variables|State|GetSelectedBuildableClass) (Variables|Grid|GetLastSnappedTransform) "Undefined" "MultiplyWithRoot" 0 false "None" 0 0 0))
                    (LocalVariables|SetNewBuildable _returnvalue)
                    (Default|PayCosts (Actor|GetComponentbyClass (Components|GetOwner) "/Game/BPs/CommonSystems/Inventory/BP_AC_Inventory.BP_AC_Inventory_C") (.BuildCosts (Utilities|GetClassDefaults (Variables|State|GetSelectedBuildableClass))))
                    (Default|IncrementBuiltCount (Variables|References|GetTrainRef) (Variables|State|GetSelectedBuildableClass))
                    (Transformation|AttachComponentToComponent (LocalVariables|GetNewBuildable) (Variables|/Game/BPs/Train/BP_TrainCompartment.BP_TrainCompartment_C|GetBuildAttachment (Variables|References|GetTargetCompartment)) "None" "KeepWorld" "KeepWorld" "KeepWorld" true)
                    (Default|MarkAreaOccupied (Variables|References|GetTargetCompartment) (Variables|Grid|GetLastCellX) (Variables|Grid|GetLastCellY) _footprintcellsx _footprintcellsy)
                    (CallFunction|ExitBuildMode)
                    (else
                      (Development|PrintString "Hello"))))
                (else
                  (Development|PrintString "Hello")
                  (CallFunction|ExitBuildMode)
                  (return)))
              (else
                (return))))
          (:else
            (return))))
      (:else
        (return)))
    (else
      (return))))