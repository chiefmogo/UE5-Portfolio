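; Player component that manages a charge resource which drains over time and can be recharged, shown on the HUD.
; Looping 0.1-second timers drive depletion and charging, with ChargePlayer switching between them and each tick pushing the percentage to the player's UI manager.
; Upgrades raise max charge while preserving the current fill ratio.
; IsActorDead reports death at zero charge but is not called here; both rate-calculation functions are empty stubs.
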(event EventBeginPlay
  (Variables|Default|SetCurrentCharge (Variables|Default|GetMaxCharge))
  (Utilities|FlowControl|Delay 0.1)
  (Variables|Default|SetPlayerUIManager (Variables|/Game/BPs/PlayerRelated/BP_Player.BP_Player_C|GetUI%20Manager%20Component (.AsBP%20Player (Utilities|Casting|CastToBP_Player (Components|GetOwner)))))
  (bind _chargepercent (CallFunction|GetChargePercent))
  (CallFunction|UpdateChargeHUD _chargepercent)
  (Utilities|Time|SetTimerbyFunctionName 0 "ChargeDepletion" 0.1 true))

(fn GetChargePercent
  (return (/ (Variables|Default|GetCurrentCharge) (Variables|Default|GetMaxCharge))))

(fn UpgradeCharge
  (params (ExtraCharge :type Float%20%28double-precision%29))
  (bind _chargepercent (CallFunction|GetChargePercent))
  (Variables|Default|SetCurrentCharge (+ (* _chargepercent ExtraCharge) (Variables|Default|GetCurrentCharge)))
  (Variables|Default|SetMaxCharge (+ (Variables|Default|GetMaxCharge) ExtraCharge)))

(fn UpdateChargeHUD
  (params (ChargePercent :type Float%20%28double-precision%29))
  (Default|UpdateHUDStats (Variables|Default|GetPlayerUIManager) "NewEnumerator0" ChargePercent))

(fn ChargeDepletion
  (Variables|Default|SetCurrentCharge (Math|Float|Clamp(Float) (- (Variables|Default|GetCurrentCharge) (* (Variables|Default|GetDepletionRatePerSecond) 0.1)) 0.0 (Variables|Default|GetMaxCharge)))
  (bind _chargepercent (CallFunction|GetChargePercent))
  (CallFunction|UpdateChargeHUD _chargepercent))

(fn CalculateChargeDepletionRate)

(fn IsActorDead
  (if (<= (Variables|Default|GetCurrentCharge) 0.0)
    (Default|PlayerDeath (Variables|Default|GetPlayerUIManager) "NewEnumerator4")))

(fn ChargePlayer
  (params (ChargePlayer? :type Boolean))
  (if ChargePlayer?
    (Class|KismetSystemLibrary|PauseTimer 0 "ChargeDepletion")
    (Utilities|Time|SetTimerbyFunctionName 0 "Charging" 0.1 true)
    (else
      (Utilities|Time|ClearTimerbyFunctionName 0 "Charging")
      (Class|KismetSystemLibrary|UnPauseTimer 0 "ChargeDepletion"))))

(fn Charging
  (Variables|Default|SetCurrentCharge (Math|Float|Clamp(Float) (+ (Variables|Default|GetCurrentCharge) (Variables|Default|GetChargingRate)) 0.0 (Variables|Default|GetMaxCharge)))
  (bind _chargepercent (CallFunction|GetChargePercent))
  (CallFunction|UpdateChargeHUD _chargepercent))

(fn CalculateChargingRate)