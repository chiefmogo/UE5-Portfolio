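; Train actor that carries a chain of compartments along a spline, with aggregate health and per-class build counts.
; BeginPlay pre-spawns all compartments below the world, hands itself to the player's building tool component, then activates the configured number.
; A movement timeline, started at zero rate, sets engine distance, and each compartment trails by accumulated lengths and spacing.
; A brake timeline scales that play rate; compartment removal is only a stub.
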(event EventBeginPlay
  (bind _returnvalue (Game|GetPlayerCharacter 0))
  (bind _tl_movement (Variables|Default|GetTL_Movement))
  (Variables|Default|SetOriginalTimelinePlayRate (/ 1.0 (Variables|Default|GetTimeForTrainToTravel)))
  (Components|Timeline|SetPlayRate _tl_movement 0.0)
  (Audio|Components|Audio|Play _tl_movement)
  (Variables|Default|SetInitialEngineOffset (+ (Variables|Default|GetCompartmentSpacing) 2025.0))
  (for _array_element (Variables|Default|GetOrderedTrainCompartmentMeshes)
    (bind _returnvalue_2 (Game|SpawnActorfromClass "/Game/BPs/Train/BP_TrainCompartment.BP_TrainCompartment_C" (Math|Transform|MakeTransform "0.0,0.0,-1000.000000" "0, 0, 0" "1.000000,1.000000,1.000000") "Undefined" "MultiplyWithRoot" 0 1.5e+02 (== _array_element "/Game/Models/Train/TrainEngine/TrainEngineV1.TrainEngineV1") 0.0 _array_element false true 0))
    (Utilities|Array|Add (Variables|Default|GetInactiveTrainCompartments) _returnvalue_2)
    (Utilities|IsValid _returnvalue :!label _label
      (:Is%20Valid
        (Variables|/Game/BPs/PlayerRelated/PlayerSystems/BP_AC_BuildingTool.BP_AC_BuildingTool_C|SetTrainRef (Actor|GetComponentbyClass _returnvalue "/Game/BPs/PlayerRelated/PlayerSystems/BP_AC_BuildingTool.BP_AC_BuildingTool_C") self))
      (:Is%20Not%20Valid
        (Utilities|FlowControl|Delay 0.2)
        (goto _label))))
  (CallFunction|MakeCompartmentActive))

(fn ConstructionScript)

(fn CalculateTotalCurrentHealth
  (for _array_element (Variables|Default|GetActiveTrainCompartments)
    (Variables|Default|SetTotalCurrentHealth (+ (Variables|/Game/BPs/Train/BP_TrainCompartment.BP_TrainCompartment_C|GetCurrentHealth _array_element) (Variables|Default|GetTotalCurrentHealth)))))

(fn CalculateTotalMaxHealth
  (for _array_element (Variables|Default|GetActiveTrainCompartments)
    (Variables|Default|SetTotalMaxHealth (+ (Variables|/Game/BPs/Train/BP_TrainCompartment.BP_TrainCompartment_C|GetMaxHealth _array_element) (Variables|Default|GetTotalMaxHealth)))))

(fn CalculateTotalHealthPercent
  (return (/ (Variables|Default|GetTotalCurrentHealth) (Variables|Default|GetTotalMaxHealth))))

(fn MoveTrainAlongSpline
  (bind _spline (Variables|Default|GetSpline))
  (bind _spline_2 (Variables|/Game/BPs/Splines/BP_Spline.BP_Spline_C|GetSpline _spline))
  (for (_array_element _array_index) (Variables|Default|GetActiveTrainCompartments)
    (LocalVariables|SetOffset (Variables|Default|GetCurrentEngineDistance))
    (for _index (range 0 (- _array_index 1))
      (LocalVariables|SetOffset (- (LocalVariables|GetOffset) (+ (Variables|/Game/BPs/Train/BP_TrainCompartment.BP_TrainCompartment_C|GetCompartmentLength (Utilities|Array|Get(acopy) (Variables|Default|GetActiveTrainCompartments) _index)) (Variables|Default|GetCompartmentSpacing)))))
    (Transformation|SetActorLocationAndRotation _array_element (Spline|GetLocationatDistanceAlongSpline _spline_2 (LocalVariables|GetOffset) "World") (Spline|GetRotationatDistanceAlongSpline _spline_2 (LocalVariables|GetOffset) "World"))))

(fn MaxCompartmentsReached
  (return (>= (Utilities|Array|Length (Variables|Default|GetActiveTrainCompartments)) (Variables|Default|GetTotalMaxCompartments))))

(fn RemoveTrainCompartment
  (params (CompartmentToRemove :type BP%20Train%20Compartment%20Object%20Reference))
  (if (== CompartmentToRemove (Utilities|Array|Get(acopy) (Variables|Default|GetActiveTrainCompartments)))
    (return)))

(fn MakeCompartmentActive
  (bind _compartmentlimitreached (CallFunction|MaxCompartmentsReached))
  (if (not _compartmentlimitreached)
    (CallFunction|SetCurrentEngineDistance (Variables|Default|GetTimelineAlphaValue))
    (for (_array_element _array_index) (Variables|Default|GetInactiveTrainCompartments)
      (if (and (not (Variables|/Game/BPs/Train/BP_TrainCompartment.BP_TrainCompartment_C|GetisActiveOnTrain _array_element)) (< _array_index (Variables|Default|GetTotalActiveTrainCompartments)))
        (Variables|/Game/BPs/Train/BP_TrainCompartment.BP_TrainCompartment_C|SetisActiveOnTrain _array_element true)
        (Utilities|Array|Add (Variables|Default|GetActiveTrainCompartments) _array_element)))
    (CallFunction|MoveTrainAlongSpline)
    (for _array_element_2 (Variables|Default|GetActiveTrainCompartments)
      (Default|InitializeCompartment _array_element_2))))

(fn SetCurrentEngineDistance
  (params (AlphaValue :type Float%20%28double-precision%29))
  (Variables|Default|SetCurrentEngineDistance (+ (* AlphaValue (- (Spline|GetSplineLength (Variables|/Game/BPs/Splines/BP_Spline.BP_Spline_C|GetSpline (Variables|Default|GetSpline))) (Variables|Default|GetInitialEngineOffset))) (Variables|Default|GetInitialEngineOffset)))
  (Variables|Default|SetTimelineAlphaValue AlphaValue))

(fn GetBuiltCount
  (params (BuildClass :type BP%20Buildables%20Master%20Class%20Reference))
  (if (Utilities|Map|Contains (Variables|Default|GetBuiltCountByClass) BuildClass)
    (return (.Value (Utilities|Map|Find (Variables|Default|GetBuiltCountByClass) BuildClass)))
    (else
      (return 0))))

(fn IncrementBuiltCount
  (params (BuildableClass :type BP%20Buildables%20Master%20Class%20Reference))
  (bind _count (CallFunction|GetBuiltCount BuildableClass))
  (bind _output_get (LocalVariables|SetCurrent _count))
  (Utilities|Map|Add (Variables|Default|GetBuiltCountByClass) BuildableClass (+ _output_get 1)))