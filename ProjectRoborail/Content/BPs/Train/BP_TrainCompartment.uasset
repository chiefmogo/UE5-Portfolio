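; BP_TrainCompartment is a train car with health and, on buildable non-engine cars, a grid surface for placing objects.
; BeginPlay sizes collision from mesh bounds and configures the build surface, marking engines unbuildable.
; Placement helpers pack cell X/Y into int64 keys to check and record occupied areas.
; The bounds check tests both axes against only the Y limits, with inverted minimum comparisons, and zero health triggers nothing.
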(event EventBeginPlay
  (bind _output_get (Variables|Default|SetCompartmentLength (* (.x (.boxextent (StaticMesh|GetBounds (Variables|Default|GetCompartmentMesh)))) 2.0)))
  (Components|Box|SetBoxExtent (Variables|Default|GetCollision) (Math|Vector|MakeVector (/ _output_get 2.0) 3e+02 3e+02) true)
  (CallFunction|SetBuildSurfaceArea))

(fn ConstructionScript)

(fn InitializeCompartment
  (Variables|Default|SetCurrentHealth (Variables|Default|GetMaxHealth))
  (Components|StaticMesh|SetStaticMesh (Variables|Default|GetSM_Compartment) (Variables|Default|GetCompartmentMesh)))

(fn TakeDamage
  (params (Damage :type Float%20%28double-precision%29))
  (bind _output_get (Variables|Default|SetCurrentHealth (Math|Float|Clamp(Float) (- (Variables|Default|GetCurrentHealth) Damage) 0.0 (Variables|Default|GetMaxHealth))))
  (if (<= _output_get 0.0)
    _))

(fn SetBuildSurfaceArea
  (if (not (Variables|Default|GetisEngine))
    (Components|Box|SetBoxExtent (Variables|Default|GetBuildSurface) "375.000000,150.000000,15.000000" true)
    (Transformation|SetRelativeLocation (Variables|Default|GetBuildSurface) "0.000000,0.000000,125.000000" false false)
    (if (not (Variables|Default|GetBuildableCompartment?))
      (Collision|SetCollisionEnabled (Variables|Default|GetBuildSurface) "NoCollision")
      (Development|SetHiddeninGame (Variables|Default|GetGridVisual) true false))
    (else
      (Components|Box|SetBoxExtent (Variables|Default|GetBuildSurface) "32.000000,32.000000,32.000000" true)
      (Transformation|SetRelativeLocation (Variables|Default|GetBuildSurface) "0.000000,0.000000,60.000000" false false)
      (Variables|Default|SetBuildableCompartment? false))))

(fn GetGridOriginTransform
  (return (Transformation|GetWorldTransform (Variables|Default|GetGridOrigin))))

(fn IsBuildable
  (return (Variables|Default|GetBuildableCompartment?)))

(fn GetBuildSurfaceComponent
  (return (Variables|Default|GetBuildSurface)))

(fn MakeCellKey
  (params (CellX :type Integer) (CellY :type Integer))
  (bind _output_get (LocalVariables|SetPackedX (+ CellX 50000)))
  (bind _output_get_2 (LocalVariables|SetPackedY (+ CellY 50000)))
  (return (Class|KismetMathLibrary|ToInt64(Integer) (+ _output_get_2 (* _output_get 100000)))))

(fn IsAreaFree?
  (params (OriginCellX :type Integer) (OriginCellY :type Integer) (SixeX :type Integer) (SizeY :type Integer))
  (for _index (range 0 (- SixeX 1))
    (LocalVariables|SetTestX (+ _index OriginCellX))
    (for _index_2 (range 0 (- SizeY 1))
      (bind _output_get (LocalVariables|SetTestY (+ _index_2 OriginCellY)))
      (bind _cellkey (CallFunction|MakeCellKey (LocalVariables|GetTestX) _output_get))
      (bind _output_get_2 (LocalVariables|SetKey _cellkey))
      (if (Utilities|Set|Contains (Variables|Default|GetOccupiedCells) _output_get_2)
        (return false))))
  (return true))

(fn MarkAreaOccupied
  (params (OriginCellX :type Integer) (OriginCellY :type Integer) (SixeX :type Integer) (SizeY :type Integer))
  (for _index (range 0 (- SixeX 1))
    (LocalVariables|SetTestX (+ _index OriginCellX))
    (for _index_2 (range 0 (- SizeY 1))
      (bind _output_get (LocalVariables|SetTestY (+ _index_2 OriginCellY)))
      (bind _cellkey (CallFunction|MakeCellKey (LocalVariables|GetTestX) _output_get))
      (bind _output_get_2 (LocalVariables|SetKey _cellkey))
      (Utilities|Set|Add (Variables|Default|GetOccupiedCells) _output_get_2))))

(fn IsAreaWithinBounds
  (params (OriginCellX :type Integer) (OriginCellY :type Integer) (SizeX :type Integer) (SizeY :type Integer))
  (LocalVariables|SetEndX (+ OriginCellX (- SizeX 1)))
  (LocalVariables|SetEndY (+ OriginCellY (- SizeY 1)))
  (return (and (and (and (>= (Variables|Default|GetMinCellY) (LocalVariables|GetEndX)) (<= (LocalVariables|GetEndX) (Variables|Default|GetMaxCellY))) (and (>= (Variables|Default|GetMinCellY) OriginCellX) (<= OriginCellX (Variables|Default|GetMaxCellY)))) (and (and (>= (Variables|Default|GetMinCellY) OriginCellY) (<= OriginCellY (Variables|Default|GetMaxCellY))) (and (>= (Variables|Default|GetMinCellY) (LocalVariables|GetEndY)) (<= (LocalVariables|GetEndY) (Variables|Default|GetMaxCellY)))))))