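; Spawns pooled world resource pickups beside the train's track as the train moves along it.
; A looping timer releases distant pickups past their grace period to the pool manager, then attempts batched spawns toward a target count.
; Candidates are random lateral offsets within a spline window around the engine, filtered by no-spawn volumes, ground trace, train distance, slope and active-pickup spacing.
; Valid spots receive a pooled pickup with weighted-random item data.
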(event EventBeginPlay
  (bind _tracksplineactor (Variables|Default|GetTrackSplineActor)
    (:then
      (Variables|Default|SetTrackSpline (Actor|GetComponentbyClass _tracksplineactor "/Script/Engine.SplineComponent"))
      (CallFunction|UpdateTrainDistance)
      (Utilities|Time|SetTimerbyFunctionName 0 "TickSpawner" (Variables|Default|GetSpawnCheckInterval) true))
    (:else)))

(fn ConstructionScript)

(fn UpdateTrainDistance
  (bind _trainactor (Variables|Default|GetTrainActor)
    (:then
      (Variables|Default|SetTrainDistanceAlongSpline (Variables|/Game/BPs/Train/BP_Train.BP_Train_C|GetCurrentEngineDistance _trainactor))
      (return))
    (:else
      (return))))

(fn TickSpawner
  (CallFunction|UpdateTrainDistance)
  (Variables|Default|GetTrackSpline
    (:then
      (Variables|Default|GetTrainActor
        (:then
          (bind _poolmanager (Variables|Default|GetPoolManager)
            (:then
              (bind _output_get (LocalVariables|SetActiveList (Variables|/Game/BPs/ResourceSpawnPool/BP_ResourcePoolManager.BP_ResourcePoolManager_C|GetActivePickups _poolmanager)))
              (for _array_element _output_get
                (if (Utilities|IsValid _array_element)
                  (if (Variables|/Game/BPs/ResourceSpawnPool/BP_WorldResourcePickup.BP_WorldResourcePickup_C|GetisActive _array_element)
                    (if (> (Math|Vector|Distance(Vector) (Transformation|GetActorLocation _array_element) (Transformation|GetActorLocation (Variables|Default|GetTrainActor))) (Variables|Default|GetDespawnRadiusWorld))
                      (bind _output_get_2 (LocalVariables|SetNow (Utilities|Time|GetGameTimeinSeconds)))
                      (bind _output_get_3 (LocalVariables|SetAge (- _output_get_2 (Variables|/Game/BPs/ResourceSpawnPool/BP_WorldResourcePickup.BP_WorldResourcePickup_C|GetSpawnTime _array_element))))
                      (if (>= _output_get_3 (Variables|/Game/BPs/ResourceSpawnPool/BP_WorldResourcePickup.BP_WorldResourcePickup_C|GetDespawnGracePeriod _array_element))
                        (Default|ReleasePickup (Variables|Default|GetPoolManager) _array_element))))))
              (if (< (Variables|/Game/BPs/ResourceSpawnPool/BP_ResourcePoolManager.BP_ResourcePoolManager_C|GetActiveCount (Variables|Default|GetPoolManager)) (Variables|Default|GetTargetActiveCount))
                (bind _output_get_4 (LocalVariables|SetToSpawn (Math|Integer|Min(Integer) (Variables|Default|GetSpawnBatchMax) (- (Variables|Default|GetTargetActiveCount) (Variables|/Game/BPs/ResourceSpawnPool/BP_ResourcePoolManager.BP_ResourcePoolManager_C|GetActiveCount (Variables|Default|GetPoolManager))))))
                (for _index (range 0 (- _output_get_4 1))
                  (CallFunction|TrySpawnOne))))
            (:else
              (return))))
        (:else
          (return))))
    (:else
      (return))))

(fn TrySpawnOne
  (bind _traceheight (Variables|Default|GetTraceHeight))
  (Variables|Default|GetTrackSpline
    (:then
      (bind _poolmanager (Variables|Default|GetPoolManager)
        (:then
          (if (!= (Utilities|Array|Length (Variables|/Game/BPs/ResourceSpawnPool/BP_ResourcePoolManager.BP_ResourcePoolManager_C|GetWorldItemDataList _poolmanager)) 0)
            (bind _output_get (LocalVariables|SetEngineD (Variables|Default|GetTrainDistanceAlongSpline)))
            (LocalVariables|SetMinD (- _output_get (Variables|Default|GetSpawnBehindDistanceAlongSpline)))
            (LocalVariables|SetMaxD (+ _output_get (Variables|Default|GetSpawnAheadDistanceAlongSpline)))
            (bind _output_get_2 (LocalVariables|SetSplineLen (Spline|GetSplineLength (Variables|Default|GetTrackSpline))))
            (LocalVariables|SetMinD (Math|Float|Clamp(Float) (LocalVariables|GetMinD) 0.0 _output_get_2))
            (LocalVariables|SetMaxD (Math|Float|Clamp(Float) (LocalVariables|GetMaxD) 0.0 _output_get_2))
            (LocalVariables|SetD (Math|Random|RandomFloatinRange (LocalVariables|GetMinD) (LocalVariables|GetMaxD)))
            (LocalVariables|SetCenter (Spline|GetLocationatDistanceAlongSpline (Variables|Default|GetTrackSpline) (LocalVariables|GetD) "World"))
            (LocalVariables|SetRight (Class|SplineComponent|GetRightVectoratDistanceAlongSpline (Variables|Default|GetTrackSpline) (LocalVariables|GetD) "World"))
            (if (Math|Random|RandomBool)
              (LocalVariables|SetSide 1)
              (else
                (LocalVariables|SetSide -1)))
            (LocalVariables|SetOffset (Math|Random|RandomFloatinRange (Variables|Default|GetMinTrackOffset) (Variables|Default|GetMaxTrackOffset)))
            (bind _output_get_3 (LocalVariables|SetCandidate (+ (LocalVariables|GetCenter) (* (LocalVariables|GetRight) (LocalVariables|GetOffset) (LocalVariables|GetSide)))))
            (bind _blocked_ (CallFunction|IsPointInsideNoSpawnVolumes _output_get_3))
            (if _blocked_
              (return false)
              (else
                (LocalVariables|SetStart (+ _output_get_3 (Math|Vector|MakeVector 0.0 0.0 _traceheight)))
                (LocalVariables|SetEnd (- _output_get_3 (Math|Vector|MakeVector 0.0 0.0 (* 2.0 _traceheight))))
                (bind (_outhit _returnvalue) (Collision|LineTraceByChannel (LocalVariables|GetStart) (LocalVariables|GetEnd) "TraceTypeQuery1" false 0 "None"))
                (if _returnvalue
                  (LocalVariables|SetHitLocation (.Location (Collision|BreakHitResult _outhit)))
                  (if (> (Math|Vector|Distance(Vector) (LocalVariables|GetHitLocation) (Transformation|GetActorLocation (Variables|Default|GetTrainActor))) (* (Variables|Default|GetDespawnRadiusWorld) 0.9))
                    (bind _output_get_4 (LocalVariables|SetSlopeDeg (Class|KismetMathLibrary|DegAcos (Math|Vector|DotProduct (.Normal (Collision|BreakHitResult _outhit)) "0.000000,0.000000,1.000000"))))
                    (if (<= _output_get_4 (Variables|Default|GetMaxSlopeDegrees))
                      (bind _outactors (Collision|SphereOverlapActors (.Location (Collision|BreakHitResult _outhit)) (Variables|Default|GetMinSpacing) (Utilities|Array|MakeArray "ObjectTypeQuery2") "/Game/BPs/ResourceSpawnPool/BP_WorldResourcePickup.BP_WorldResourcePickup_C" (Utilities|Array|MakeArray self)))
                      (if (> (Utilities|Array|Length _outactors) 0)
                        (for _array_element _outactors
                          (bind _asbp_world_resource_pickup (Utilities|Casting|CastToBP_WorldResourcePickup _array_element)
                            (:then
                              (if (not (Variables|/Game/BPs/ResourceSpawnPool/BP_WorldResourcePickup.BP_WorldResourcePickup_C|GetisActive _asbp_world_resource_pickup))
                                (bind _pickup (Default|AcquirePickup (Variables|Default|GetPoolManager)))
                                (bind _output_get_5 (LocalVariables|SetPickup _pickup))
                                (if (not (Utilities|IsValid _output_get_5))
                                  (return false)
                                  (else
                                    (bind _itemdata (Default|SelectWeightedItem (Variables|Default|GetPoolManager)))
                                    (Utilities|IsValid _itemdata
                                      (:Is%20Valid
                                        (LocalVariables|SetItemData _itemdata)
                                        (Transformation|SetActorLocation (LocalVariables|GetPickup) (LocalVariables|GetHitLocation) false false)
                                        (Default|ActivatePickup (LocalVariables|GetPickup) (LocalVariables|GetItemData) (Variables|Default|GetPoolManager))
                                        (Default|RegisterActivePickup (Variables|Default|GetPoolManager))
                                        (return true))
                                      (:Is%20Not%20Valid
                                        (return false)))))
                                (else
                                  (return false))))
                            (:CastFailed
                              (return false))))
                        (else
                          (bind _pickup_2 (Default|AcquirePickup (Variables|Default|GetPoolManager)))
                          (bind _output_get_6 (LocalVariables|SetPickup _pickup_2))
                          (if (not (Utilities|IsValid _output_get_6))
                            (return false)
                            (else
                              (bind _itemdata_2 (Default|SelectWeightedItem (Variables|Default|GetPoolManager)))
                              (Utilities|IsValid _itemdata_2
                                (:Is%20Valid
                                  (LocalVariables|SetItemData _itemdata_2)
                                  (Transformation|SetActorLocation (LocalVariables|GetPickup) (LocalVariables|GetHitLocation) false false)
                                  (Default|ActivatePickup (LocalVariables|GetPickup) (LocalVariables|GetItemData) (Variables|Default|GetPoolManager))
                                  (Default|RegisterActivePickup (Variables|Default|GetPoolManager) (LocalVariables|GetPickup))
                                  (return true))
                                (:Is%20Not%20Valid
                                  (return false)))))))
                      (else
                        (return false)))
                    (else
                      (return false)))
                  (else
                    (return false)))))
            (else
              (return false))))
        (:else
          (return false))))
    (:else
      (return false))))

(fn IsPointInsideNoSpawnVolumes
  (params (Point :type Vector))
  (for _array_element (Variables|Default|GetNoSpawnVolumes)
    (Utilities|IsValid _array_element
      (:Is%20Valid
        (if (== (.ReturnValue (Collision|GetClosestPointonCollision _array_element Point "None")) 0.0)
          (return true)))))
  (return false))