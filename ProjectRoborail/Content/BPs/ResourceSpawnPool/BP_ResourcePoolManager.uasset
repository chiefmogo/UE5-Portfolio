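; BP_ResourcePoolManager is an object pool for world resource pickup actors, paired with weighted random selection of the item data they can use.
; BeginPlay prewarms deactivated pickups into an inactive list, which AcquirePickup pops from the end without growing when empty.
; Registration tracks active pickups, while release deactivates them, moves them far below the world and returns them to the pool.
; Item selection uses a cached total spawn weight, recalculated when dirty.
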(event EventBeginPlay
  (CallFunction|CleanupActivePickups)
  (for _index (range 0 (- (Variables|Default|GetPrewarmCount) 1))
    (bind _returnvalue (Game|SpawnActorfromClass "/Game/BPs/ResourceSpawnPool/BP_WorldResourcePickup.BP_WorldResourcePickup_C" (Math|Transform|MakeTransform "0, 0, 0" "0, 0, 0" "1.000000,1.000000,1.000000") "Undefined" "MultiplyWithRoot" 0 0 0))
    (Default|DeactivatePickup _returnvalue)
    (Variables|/Game/BPs/ResourceSpawnPool/BP_WorldResourcePickup.BP_WorldResourcePickup_C|SetPoolManager _returnvalue self)
    (Utilities|Array|Add (Variables|Default|GetInactive) _returnvalue)))

(fn ConstructionScript)

(fn AcquirePickup
  (bind _inactive (Variables|Default|GetInactive))
  (bind _inactive_2 (Variables|Default|GetInactive))
  (bind _returnvalue (Utilities|Array|LastIndex _inactive))
  (bind _output (Utilities|Array|Get(acopy) _inactive _returnvalue))
  (if (> (Utilities|Array|Length (Variables|Default|GetInactive)) 0)
    (Utilities|IsValid _output
      (:Is%20Valid
        (LocalVariables|SetPickupTemp _output)
        (Utilities|Array|RemoveIndex _inactive_2 (Utilities|Array|LastIndex _inactive_2))
        (return (LocalVariables|GetPickupTemp)))
      (:Is%20Not%20Valid
        (return 0)))
    (else
      (return 0))))

(fn ReleasePickup
  (params (Pickup :type BP%20World%20Resource%20Pickup%20Object%20Reference))
  (Utilities|IsValid Pickup
    (:Is%20Valid
      (Default|DeactivatePickup Pickup)
      (Utilities|Array|RemoveItem (Variables|Default|GetActivePickups) Pickup)
      (Variables|Default|SetActiveCount (Utilities|Array|Length (Variables|Default|GetActivePickups)))
      (Transformation|SetActorLocation Pickup "0.000000,0.000000,-100000.000000" false false)
      (Utilities|Array|RemoveItem (Variables|Default|GetInactive) Pickup)
      (Utilities|Array|Add (Variables|Default|GetInactive) Pickup)
      (Variables|Default|SetActiveCount (Math|Integer|Max(Integer) (- (Variables|Default|GetActiveCount) 1)))
      (return))
    (:Is%20Not%20Valid
      (return))))

(fn RecalculateTotalSpawnWeight
  (Variables|Default|SetTotalSpawnWeight 0.0)
  (for _array_element (Variables|Default|GetWorldItemDataList)
    (Utilities|IsValid _array_element
      (:Is%20Valid
        (if (> (Variables|/Game/BPs/ResourceCollectibles/DataAssets/PDA_Collectibles.PDA_Collectibles_C|GetResourceSpawnWeight _array_element) 0.0)
          (Variables|Default|SetTotalSpawnWeight (+ (Variables|Default|GetTotalSpawnWeight) (Variables|/Game/BPs/ResourceCollectibles/DataAssets/PDA_Collectibles.PDA_Collectibles_C|GetResourceSpawnWeight _array_element)))))))
  (Variables|Default|SetWeightsDirty false))

(fn SelectWeightedItem
  (if (!= (Utilities|Array|Length (Variables|Default|GetWorldItemDataList)) 0)
    (if (or (Variables|Default|GetWeightsDirty) (<= (Variables|Default|GetTotalSpawnWeight) 0.0))
      (CallFunction|RecalculateTotalSpawnWeight))
    (if (> (Variables|Default|GetTotalSpawnWeight) 0.0)
      (LocalVariables|SetRand (Math|Random|RandomFloatinRange 0.0 (Variables|Default|GetTotalSpawnWeight)))
      (bind _array_element (Utilities|Array|ForEachLoopwithBreak (Variables|Default|GetWorldItemDataList))
        (:LoopBody
          (Utilities|IsValid _array_element
            (:Is%20Valid
              (if (> (Variables|/Game/BPs/ResourceCollectibles/DataAssets/PDA_Collectibles.PDA_Collectibles_C|GetResourceSpawnWeight _array_element) 0.0)
                (bind _output_get (LocalVariables|SetRunningSum (+ (LocalVariables|GetRunningSum) (Variables|/Game/BPs/ResourceCollectibles/DataAssets/PDA_Collectibles.PDA_Collectibles_C|GetResourceSpawnWeight _array_element))))
                (if (>= _output_get (LocalVariables|GetRand))
                  (return _array_element)))))))
      (else
        (return 0)))
    (else
      (return 0))))

(fn ChangeSpawnWeight)

(fn RegisterActivePickup
  (params (Pickup :type BP%20World%20Resource%20Pickup%20Object%20Reference))
  (Utilities|IsValid Pickup
    (:Is%20Valid
      (if (not (Utilities|Array|ContainsItem (Variables|Default|GetActivePickups) Pickup))
        (Utilities|Array|Add (Variables|Default|GetActivePickups) Pickup)
        (Variables|Default|SetActiveCount (Utilities|Array|Length (Variables|Default|GetActivePickups)))))
    (:Is%20Not%20Valid
      (return))))

(fn CleanupActivePickups
  (bind _output_get (LocalVariables|SetActivePickupsLocalCopy (Variables|Default|GetActivePickups)))
  (for _array_element _output_get
    (Utilities|IsValid _array_element
      (:Is%20Valid
        (CallFunction|ReleasePickup _array_element))))
  (Utilities|Array|Clear (Variables|Default|GetActivePickups))
  (Variables|Default|SetActiveCount 0))