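; Base Blueprint for placeable buildables that can offer an interaction UI.
; On BeginPlay, buildables flagged NeedsInteractionUI add Interactable and FacingCharacter tags to themselves.
; The Interact event casts the first player character to BP_Player and has its UIManagerComponent open the buildable UI for this actor.
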(event EventBeginPlay
  (bind _tags (Variables|Actor|GetTags))
  (if (Variables|Default|GetNeedsInteractionUI)
    (Utilities|Array|AddUnique _tags "Interactable")
    (Utilities|Array|AddUnique _tags "FacingCharacter")))

(event Collision|EventActorBeginOverlap
  (params (OtherActor :type Actor%20Object%20Reference)))

(event EventTick
  (params (DeltaSeconds :type Float%20%28single-precision%29)))

(event EventInteract
  (Default|OpenBuildableUI (Variables|/Game/BPs/PlayerRelated/BP_Player.BP_Player_C|GetUI%20Manager%20Component (.AsBP%20Player (Utilities|Casting|CastToBP_Player (Game|GetPlayerCharacter 0)))) self))

(fn ConstructionScript)