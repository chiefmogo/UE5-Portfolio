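; BP_BuildPreviewActor is a preview actor for building that displays a static mesh with a valid or invalid look.
; SetPreviewMesh swaps the mesh on the PreviewMesh component, and SetValidState sets its first material slot to MIValid or MIInvalid from a boolean.
; It has no logic of its own in the event graph or construction script, so both functions rely on outside callers.
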(event EventBeginPlay)

(event Collision|EventActorBeginOverlap
  (params (OtherActor :type Actor%20Object%20Reference)))

(event EventTick
  (params (DeltaSeconds :type Float%20%28single-precision%29)))

(fn ConstructionScript)

(fn SetPreviewMesh
  (params (InMesh :type Static%20Mesh%20Object%20Reference))
  (Components|StaticMesh|SetStaticMesh (Variables|Default|GetPreviewMesh) InMesh))

(fn SetValidState
  (params (Valid :type Boolean))
  (bind _previewmesh (Variables|Default|GetPreviewMesh))
  (if Valid
    (Rendering|Material|SetMaterial _previewmesh 0 (Variables|Default|GetMI_Valid))
    (else
      (Rendering|Material|SetMaterial _previewmesh 0 (Variables|Default|GetMI_Invalid)))))