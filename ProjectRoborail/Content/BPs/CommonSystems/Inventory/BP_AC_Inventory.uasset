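; Slot-based inventory component that stores stackable items, tracks carry weight and overweight ratio, and handles build costs.
; Adds fill partial stacks before empty slots; changed slots are sanitized against stack limits, and mutations recalculate weight and fire slot, inventory and weight events.
; Cost checks total items across slots, while payment deducts each cost sequentially without rollback.
; Transfers add to the target first, then remove from the source, with a compensating target removal on shortfall.
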(event EventBeginPlay
  (CallFunction|InitializeSlots (Variables|Default|GetDefaultSlots) false))

(fn IsSlotEmpty?
  (params (Slot :type S%20Inventory%20Slot%20Structure))
  (bind (_itemdata _itemquantity) (Utilities|Struct|BreakS_InventorySlot Slot))
  (return (or (== _itemdata 0) (<= _itemquantity 0))))

(fn GetMaxStack
  (params (ItemData :type PDA%20Collectibles%20Object%20Reference))
  (if (== ItemData 0)
    (return 0)
    (elif (Variables|/Game/BPs/ResourceCollectibles/DataAssets/PDA_Collectibles.PDA_Collectibles_C|GetStackable ItemData)
      (return (Math|Integer|Max(Integer) 1 (Variables|/Game/BPs/ResourceCollectibles/DataAssets/PDA_Collectibles.PDA_Collectibles_C|GetResourceMaxStackSize ItemData)))
      (else
        (return 1)))))

(fn GetUnitWeight
  (params (ItemData :type PDA%20Collectibles%20Object%20Reference))
  (if (!= ItemData 0)
    (return (Math|Float|Max(Float) 0.0 (Variables|/Game/BPs/ResourceCollectibles/DataAssets/PDA_Collectibles.PDA_Collectibles_C|GetResourceWeight ItemData)))
    (else
      (return 0.0))))

(fn SanitizeSlot
  (params (InSlot :type S%20Inventory%20Slot%20Structure))
  (LocalVariables|SetSlot InSlot)
  (if (not (Utilities|IsValid (.ItemData (Utilities|Struct|BreakS_InventorySlot (LocalVariables|GetSlot)))))
    (bind _output_get (LocalVariables|SetSlot (Utilities|Struct|MakeS_InventorySlot 0 0)))
    (return _output_get)
    (elif (<= (.ItemQuantity (Utilities|Struct|BreakS_InventorySlot (LocalVariables|GetSlot))) 0)
      (bind _output_get_2 (LocalVariables|SetSlot (Utilities|Struct|MakeS_InventorySlot 0 0)))
      (return _output_get_2)
      (else
        (bind _output_get_3 (LocalVariables|SetSlot (Utilities|Struct|MakeS_InventorySlot (.ItemData (Utilities|Struct|BreakS_InventorySlot (LocalVariables|GetSlot))) (Math|Integer|Min(Integer) (.ItemQuantity (Utilities|Struct|BreakS_InventorySlot (LocalVariables|GetSlot))) (CallFunction|GetMaxStack (.ItemData (Utilities|Struct|BreakS_InventorySlot (LocalVariables|GetSlot))))))))
        (return _output_get_3)))))

(fn SanitizeAllSlots
  (for _index (range 0 (- (Utilities|Array|Length (Variables|Default|GetSlots)) 1))
    (bind _sanitizedslot (CallFunction|SanitizeSlot (Utilities|Array|Get(acopy) (Variables|Default|GetSlots) _index)))
    (Utilities|Array|SetArrayElem (Variables|Default|GetSlots) _index _sanitizedslot)))

(fn RecalculateWeightandBroadcast
  (LocalVariables|SetNewWeight 0.0)
  (for _array_element (Variables|Default|GetSlots)
    (LocalVariables|SetNewWeight (+ (* (CallFunction|GetUnitWeight (.ItemData (Utilities|Struct|BreakS_InventorySlot _array_element))) (Math|Conversions|ToFloat(Integer) (.ItemQuantity (Utilities|Struct|BreakS_InventorySlot _array_element)))) (LocalVariables|GetNewWeight))))
  (Variables|Default|SetCurrentWeight (LocalVariables|GetNewWeight))
  (if (<= (Variables|Default|GetBaseCarryWeight) 0.0)
    (Variables|Default|SetOverweightRatio 0.0)
    (else
      (Variables|Default|SetOverweightRatio (Math|Float|Max(Float) 0.0 (/ (- (Variables|Default|GetCurrentWeight) (Variables|Default|GetBaseCarryWeight)) (Variables|Default|GetBaseCarryWeight))))))
  (Default|CallOnWeightChanged (Variables|Default|GetCurrentWeight) (Variables|Default|GetOverweightRatio)))

(fn InitializeSlots
  (params (InDefaultSlots :type Integer) (PreserveExisting :type Boolean))
  (Variables|Default|SetDefaultSlots (Math|Integer|Max(Integer) InDefaultSlots))
  (if (<= (Variables|Default|GetCurrentMaxSlots) 0)
    (Variables|Default|SetCurrentMaxSlots (Variables|Default|GetDefaultSlots)))
  (if PreserveExisting
    (Utilities|Array|Resize (Variables|Default|GetSlots) (Variables|Default|GetCurrentMaxSlots))
    (else
      (Utilities|Array|Clear (Variables|Default|GetSlots))
      (for _index (range 0 (- (Variables|Default|GetCurrentMaxSlots) 1))
        (Utilities|Array|Add (Variables|Default|GetSlots) (Utilities|Struct|MakeS_InventorySlot 0)))))
  (CallFunction|SanitizeAllSlots)
  (CallFunction|RecalculateWeightandBroadcast)
  (Default|CallOnInventoryChanged))

(fn TryAdd
  (params (Item%20Data :type PDA%20Collectibles%20Object%20Reference) (QuantityToAdd :type Integer))
  (LocalVariables|SetLocalAdded 0)
  (LocalVariables|SetLocalRemaining (Math|Integer|Max(Integer) 0 QuantityToAdd))
  (LocalVariables|GetItem%20Data
    (:then
      (if (> (LocalVariables|GetLocalRemaining) 0)
        (LocalVariables|SetMaxStack (CallFunction|GetMaxStack Item%20Data))
        (bind _index (Utilities|FlowControl|ForLoopwithBreak 0 (- (Utilities|Array|Length (Variables|Default|GetSlots)) 1) :!pinned true :!label _label) ; Pass 1 - Fill Partial Slots
          (:LoopBody
            (bind _output_get (LocalVariables|SetSlotCopy (Utilities|Array|Get(acopy) (Variables|Default|GetSlots) _index)))
            (if (== (.ItemData (Utilities|Struct|BreakS_InventorySlot _output_get)) Item%20Data)
              (bind _output_get_2 (LocalVariables|SetSpace (- (LocalVariables|GetMaxStack) (.ItemQuantity (Utilities|Struct|BreakS_InventorySlot _output_get)))))
              (if (> _output_get_2 0)
                (bind _output_get_3 (LocalVariables|SetToMove (Math|Integer|Min(Integer) (LocalVariables|GetSpace) (LocalVariables|GetLocalRemaining))))
                (if (> _output_get_3 0)
                  (LocalVariables|SetSlotCopy (Utilities|Struct|MakeS_InventorySlot (.itemdata (LocalVariables|GetSlotCopy)) (+ (.itemquantity (LocalVariables|GetSlotCopy)) (LocalVariables|GetToMove))))
                  (LocalVariables|SetLocalAdded (+ (LocalVariables|GetLocalAdded) (LocalVariables|GetToMove)))
                  (LocalVariables|SetLocalRemaining (- (LocalVariables|GetLocalRemaining) (LocalVariables|GetToMove)))
                  (bind _sanitizedslot (CallFunction|SanitizeSlot (LocalVariables|GetSlotCopy)))
                  (Utilities|Array|SetArrayElem (Variables|Default|GetSlots) _index _sanitizedslot)
                  (Default|CallOnSlotChanged _index)
                  (if (<= (LocalVariables|GetLocalRemaining) 0)
                    (goto _label Break))))))
          (:Completed
            (if (> (LocalVariables|GetLocalRemaining) 0)
              (bind _index_2 (Utilities|FlowControl|ForLoopwithBreak 0 (- (Utilities|Array|Length (Variables|Default|GetSlots)) 1) :!pinned true :!label _label_2) ; Pass 2 - Fill Empty Slots
                (:LoopBody
                  (bind _output_get_4 (LocalVariables|SetSlotCopy2 (Utilities|Array|Get(acopy) (Variables|Default|GetSlots) _index_2)))
                  (if (CallFunction|IsSlotEmpty? _output_get_4)
                    (bind _output_get_5 (LocalVariables|SetToMove (Math|Integer|Min(Integer) (LocalVariables|GetMaxStack) (LocalVariables|GetLocalRemaining))))
                    (if (> _output_get_5 0)
                      (LocalVariables|SetSlotCopy2 (Utilities|Struct|MakeS_InventorySlot Item%20Data (LocalVariables|GetToMove)))
                      (LocalVariables|SetLocalAdded (+ (LocalVariables|GetLocalAdded) (LocalVariables|GetToMove)))
                      (LocalVariables|SetLocalRemaining (- (LocalVariables|GetLocalRemaining) (LocalVariables|GetToMove)))
                      (bind _sanitizedslot_2 (CallFunction|SanitizeSlot (LocalVariables|GetSlotCopy2)))
                      (Utilities|Array|SetArrayElem (Variables|Default|GetSlots) _index_2 _sanitizedslot_2)
                      (Default|CallOnSlotChanged _index_2)
                      (if (<= (LocalVariables|GetLocalRemaining) 0)
                        (goto _label_2 Break)))))
                (:Completed
                  (if (> (LocalVariables|GetLocalAdded) 0) :!label _label_3
                    (CallFunction|RecalculateWeightandBroadcast)
                    (Default|CallOnInventoryChanged))
                  (return (LocalVariables|GetLocalAdded) (LocalVariables|GetLocalRemaining) (> (LocalVariables|GetLocalAdded) 0))))
              (else
                (goto _label_3)))))
        (else
          (return 0 0 false))))
    (:else
      (return 0 0 false))))

(fn TryRemovefromSlot
  (params (SlotIndex :type Integer) (QuantityToRemove :type Integer))
  (LocalVariables|SetLocalRemoved 0)
  (bind _output_get (LocalVariables|SetLocalToRemove (Math|Integer|Max(Integer) 0 QuantityToRemove)))
  (if (<= _output_get 0)
    (return 0 false)
    (elif (or (< SlotIndex 0) (>= SlotIndex (Utilities|Array|Length (Variables|Default|GetSlots))))
      (return 0 false)
      (else
        (bind _output_get_2 (LocalVariables|SetSlotCopy (Utilities|Array|Get(acopy) (Variables|Default|GetSlots) SlotIndex)))
        (if (CallFunction|IsSlotEmpty? _output_get_2)
          (return 0 false)
          (else
            (bind _output_get_3 (LocalVariables|SetSlotQty (.ItemQuantity (Utilities|Struct|BreakS_InventorySlot (LocalVariables|GetSlotCopy)))))
            (bind _output_get_4 (LocalVariables|SetToRemove (Math|Integer|Min(Integer) _output_get_3 (LocalVariables|GetLocalToRemove))))
            (if (<= _output_get_4 0)
              (return 0 false)
              (else
                (bind _output_get_5 (LocalVariables|SetNewQty (- (LocalVariables|GetSlotQty) (LocalVariables|GetToRemove))))
                (bind _output_get_6 (LocalVariables|SetSlotCopy (Utilities|Struct|MakeS_InventorySlot (.itemdata (LocalVariables|GetSlotCopy)) _output_get_5)))
                (bind _sanitizedslot (CallFunction|SanitizeSlot _output_get_6))
                (Utilities|Array|SetArrayElem (Variables|Default|GetSlots) SlotIndex _sanitizedslot)
                (bind _output_get_7 (LocalVariables|SetLocalRemoved (LocalVariables|GetToRemove)))
                (if (> _output_get_7 0)
                  (Default|CallOnSlotChanged SlotIndex)
                  (CallFunction|RecalculateWeightandBroadcast)
                  (Default|CallOnInventoryChanged)
                  (return (LocalVariables|GetLocalRemoved) (> (LocalVariables|GetLocalRemoved) 0)))))))))))

(fn TryRemovebyItem
  (params (ItemData :type PDA%20Collectibles%20Object%20Reference) (QuantityToRemove :type Integer))
  (LocalVariables|SetLocalRemoved 0)
  (LocalVariables|SetLocalRemaining (Math|Integer|Max(Integer) 0 QuantityToRemove))
  (LocalVariables|SetAnySlotChanged false)
  (if (not (Utilities|IsValid ItemData))
    (return 0 0 false)
    (elif (<= (LocalVariables|GetLocalRemaining) 0)
      (return 0 0 false)
      (else
        (bind _index (Utilities|FlowControl|ForLoopwithBreak 0 (- (Utilities|Array|Length (Variables|Default|GetSlots)) 1) :!label _label)
          (:LoopBody
            (if (<= (LocalVariables|GetLocalRemaining) 0)
              (goto _label Break)
              (else
                (bind _output_get (LocalVariables|SetSlotCopy (Utilities|Array|Get(acopy) (Variables|Default|GetSlots) _index)))
                (if (== (.ItemData (Utilities|Struct|BreakS_InventorySlot _output_get)) ItemData)
                  (if (not (<= (.ItemQuantity (Utilities|Struct|BreakS_InventorySlot _output_get)) 0))
                    (bind _output_get_2 (LocalVariables|SetToRemove (Math|Integer|Min(Integer) (.ItemQuantity (Utilities|Struct|BreakS_InventorySlot _output_get)) (LocalVariables|GetLocalRemaining))))
                    (bind _output_get_3 (LocalVariables|SetNewQty (- (.itemquantity (LocalVariables|GetSlotCopy)) _output_get_2)))
                    (LocalVariables|SetSlotCopy (Utilities|Struct|MakeS_InventorySlot (.itemdata (LocalVariables|GetSlotCopy)) _output_get_3))
                    (LocalVariables|SetLocalRemoved (+ (LocalVariables|GetLocalRemoved) (LocalVariables|GetToRemove)))
                    (LocalVariables|SetLocalRemaining (- (LocalVariables|GetLocalRemaining) (LocalVariables|GetToRemove)))
                    (bind _sanitizedslot (CallFunction|SanitizeSlot (LocalVariables|GetSlotCopy)))
                    (Utilities|Array|SetArrayElem (Variables|Default|GetSlots) _index _sanitizedslot)
                    (Default|CallOnSlotChanged _index)
                    (LocalVariables|SetAnySlotChanged true)
                    (if (<= (LocalVariables|GetLocalRemaining) 0)
                      (goto _label Break)))))))
          (:Completed
            (if (LocalVariables|GetAnySlotChanged)
              (CallFunction|RecalculateWeightandBroadcast)
              (Default|CallOnInventoryChanged))
            (return (LocalVariables|GetLocalRemoved) (LocalVariables|GetLocalRemaining) (== (LocalVariables|GetLocalRemaining) 0))))))))

(fn GetTotalQuantity
  (params (ItemData :type PDA%20Collectibles%20Object%20Reference))
  (if (not (Utilities|IsValid ItemData))
    (return 0)
    (else
      (LocalVariables|SetTotal 0)
      (for _array_element (Variables|Default|GetSlots)
        (if (== (.ItemData (Utilities|Struct|BreakS_InventorySlot _array_element)) ItemData)
          (LocalVariables|SetTotal (+ (LocalVariables|GetTotal) (.ItemQuantity (Utilities|Struct|BreakS_InventorySlot _array_element))))))
      (return (LocalVariables|GetTotal)))))

(fn HasItems
  (params (ItemData :type PDA%20Collectibles%20Object%20Reference) (QuantityNeeded :type Integer))
  (if (Utilities|IsValid ItemData)
    (if (<= QuantityNeeded 0)
      (return true)
      (else
        (bind _output_get (LocalVariables|SetTotal (CallFunction|GetTotalQuantity ItemData)))
        (return (>= _output_get QuantityNeeded))))
    (else
      (return false))))

(fn CanAffordCosts
  (params (BuildCosts :type Array%20of%20S%20Build%20Cost%20Entry%20Structures))
  (if (== (Utilities|Array|Length BuildCosts) 0)
    (return true)
    (else
      (for _array_element BuildCosts
        (if (not (or (not (Utilities|IsValid (.ItemID (Utilities|Struct|BreakS_BuildCostEntry _array_element)))) (<= (.ItemAmount (Utilities|Struct|BreakS_BuildCostEntry _array_element)) 0)))
          (if (not (CallFunction|HasItems (.ItemID (Utilities|Struct|BreakS_BuildCostEntry _array_element)) (.ItemAmount (Utilities|Struct|BreakS_BuildCostEntry _array_element))))
            (return false))))
      (return true))))

(fn PayCosts
  (params (BuildCosts :type Array%20of%20S%20Build%20Cost%20Entry%20Structures))
  (for _array_element BuildCosts
    (if (not (or (not (Utilities|IsValid (.ItemID (Utilities|Struct|BreakS_BuildCostEntry _array_element)))) (<= (.ItemAmount (Utilities|Struct|BreakS_BuildCostEntry _array_element)) 0)))
      (bind _quantityremaining (CallFunction|TryRemovebyItem (.ItemID (Utilities|Struct|BreakS_BuildCostEntry _array_element)) (.ItemAmount (Utilities|Struct|BreakS_BuildCostEntry _array_element))))
      (if (> _quantityremaining 0)
        (return false))))
  (return true))

(fn Transferto
  (params (TargetInventory :type BP%20AC%20Inventory%20Object%20Reference) (ItemData :type PDA%20Collectibles%20Object%20Reference) (QunatityToTransfer :type Integer))
  (LocalVariables|SetLocalTransferred 0)
  (LocalVariables|SetLocalRemaining (Math|Integer|Max(Integer) 0 QunatityToTransfer))
  (bind _targetinventory (LocalVariables|GetTargetInventory)
    (:then
      (if (!= _targetinventory self)
        (LocalVariables|GetItemData
          (:then
            (if (> (LocalVariables|GetLocalRemaining) 0)
              (bind (_quantityadded _quantityremaining _success) (CallFunction|TryAdd TargetInventory ItemData (LocalVariables|GetLocalRemaining)))
              (bind _output_get (LocalVariables|SetTargetAdded _quantityadded))
              (LocalVariables|SetTargetRemaining _quantityremaining)
              (LocalVariables|SetTargetSuccess _success)
              (if (> _output_get 0)
                (bind (_quantityremoved _quantityremaining_2 _success_2) (CallFunction|TryRemovebyItem ItemData (LocalVariables|GetTargetAdded)))
                (LocalVariables|SetRemoveRemoved _quantityremoved)
                (bind _output_get_2 (LocalVariables|SetRemoveRemaining _quantityremaining_2))
                (LocalVariables|SetRemoveSuccess _success_2)
                (if (== _output_get_2 0)
                  (bind _output_get_3 (LocalVariables|SetLocalTransferred (LocalVariables|GetTargetAdded)))
                  (LocalVariables|SetLocalRemaining (- (LocalVariables|GetLocalRemaining) _output_get_3))
                  (return (LocalVariables|GetLocalTransferred) (LocalVariables|GetLocalRemaining) (> (LocalVariables|GetLocalTransferred) 0))
                  (else
                    (CallFunction|TryRemovebyItem TargetInventory ItemData (LocalVariables|GetRemoveRemoved))
                    (return 0 (LocalVariables|GetLocalRemaining) false)))
                (else
                  (return 0 (LocalVariables|GetLocalRemaining) false)))
              (else
                (return 0 0 false))))
          (:else
            (return 0 (LocalVariables|GetLocalRemaining) false)))
        (else
          (return 0 (LocalVariables|GetLocalRemaining) false))))
    (:else
      (return 0 (LocalVariables|GetLocalRemaining) false))))

(fn GetSlot
  (params (SlotIndex :type Integer))
  (if (or (< SlotIndex 0) (>= SlotIndex (Utilities|Array|Length (Variables|Default|GetSlots))))
    (return "")
    (else
      (return (Utilities|Array|Get(acopy) (Variables|Default|GetSlots) SlotIndex)))))